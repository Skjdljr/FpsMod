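; Base weapon Blueprint that a MyChar picks up by overlapping it, with mostly empty hooks for firing and reloading.
; Overlap runs ServerEquip, which registers the weapon on the character and snaps it to WeaponComponent, while UnEquip detaches it through ServerUnEquip, both tracked by Attached.
; Shooting only prints a debug string after calling the empty AttemptShoot.
; Melee plays a WeaponSwing timeline whose mesh rotation delta is currently zero.
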(event `self.ReceiveBeginPlay`)

(event `self.ReceiveActorBeginOverlap`
  (params (OtherActor :type "Actor Object Reference"))
  (`self.ServerEquip` OtherActor))

(event `ServerEquip`
  (params (Pawn :type "Actor Object Reference"))
  (`self.OnServerEquip` Pawn))

(event `ServerUnEquip`
  (if (`self.bAttached`)
    (`self.DetachRootComponentFromParent` true)
    (set `self.bAttached` false)))

(event `ServerAttemptShoot`
  (`self.AttemptShoot`)
  (`KismetSystemLibrary.PrintString` "Shoot that"))

(event `Melee`
  (`Timeline|WeaponSwing`
    (:`Update`
      (`SceneComponent.K2_AddLocalRotation` (`self.WeaponMesh`) (`KismetMathLibrary.MakeRot` 0.0) false))))

(fn `AttemptShoot`)

(fn `CanFire`)

(fn `CanReload`)

(fn `GetAmmoType`
  (returns (NewParam :type "/Game/Blueprints/Weapons/AmmoType Enum"))
  (bind (_weaponinfo_battached _weaponinfo_binfinteammo _weaponinfo_maxammo _weaponinfo_ammoperclip _weaponinfo_initialclips _weaponinfo_timebetweenshots _weaponinfo_reloadduration _weaponinfo_ammotype) (break `/Game/Blueprints/Weapons/WeaponInfo` (`self.WeaponInfo`)))
  (return _weaponinfo_ammotype))

(fn `HasAmmo`)

(fn `IsAttachedToPawn`
  (returns (attached :type Boolean))
  (return (`self.bAttached`)))

(fn `OnServerEquip`
  (params (pawn :type "Actor Object Reference"))
  (if (not (`self.bAttached`))
    (bind _asmy_char (cast `/Game/Blueprints/MyChar` pawn))
    (bind _output_get (set `self.MyPawn` _asmy_char))
    (`/Game/Blueprints/MyChar.SetWeapon` _output_get self)
    (`SceneComponent.K2_AttachTo` (`/Game/Blueprints/MyChar.WeaponComponent` (`self.MyPawn`)) "None" "SnapToTarget")
    (set `self.bAttached` true)))

(fn `StopFire`)

(fn `StopReload`)

(fn `TryReload`)

(fn `UnEquip`
  (`self.ServerUnEquip`))

(fn `UserConstructionScript`)