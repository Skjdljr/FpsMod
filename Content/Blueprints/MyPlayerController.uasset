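; Player controller that handles spell quick-bar input, the spell sheet window and HUD messaging.
; Seven quick-bar actions set a shared slot index, notify the HUD, and on press ask MyChar's server to use that PlayerSpells entry.
; P toggles the SpellSheet widget with cursor and input mode, while G unequips the primary weapon.
; SetPlayerSpells refreshes the HUD spell bar, and UpdateHud sends hardcoded ammo and health values.
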(event `self.ReceiveBeginPlay`)

(event `InputAction|QuickBar1`
  (bind _returnvalue (`self.GetHUD`))
  (bind _index (`self.Index`))
  ;[1 1 1] Input
  (:`Pressed`
    (set `self.index` 0)
    (message `/Game/Blueprints/HUD/UIInterface.QuickBarPressed` _returnvalue _index :!label _label)
    ;[1 0.4811 0.2378] Use spell
    (bind _asmy_char (`self.GetMyChar`))
    (bind (_item _canuse) (`self.HasSpellToUse`))
    (if _canuse
      (`/Game/Blueprints/MyChar.ServerAttemptToUseSpell` _asmy_char _item)
      (else
        (`KismetSystemLibrary.PrintString` "Please equip a spell to use" true true (struct :`R` 1.0 :`G` 0.18712 :`B` 0.072207 :`A` 1.0)))))
  (:`Released`
    (set `self.index` 0)
    (message `/Game/Blueprints/HUD/UIInterface.QuickBarReleased` _returnvalue _index :!label _label_2)))

(event `InputAction|QuickBar2`
  ;[1 1 1] Input
  (:`Pressed`
    (set `self.index` 1)
    (goto _label))
  (:`Released`
    (set `self.index` 1)
    (goto _label_2)))

(event `InputAction|QuickBar3`
  ;[1 1 1] Input
  (:`Pressed`
    (set `self.index` 2)
    (goto _label))
  (:`Released`
    (set `self.index` 2)
    (goto _label_2)))

(event `InputAction|QuickBar4`
  ;[1 1 1] Input
  (:`Pressed`
    (set `self.index` 3)
    (goto _label))
  (:`Released`
    (set `self.index` 3)
    (goto _label_2)))

(event `InputAction|QuickBar5`
  ;[1 1 1] Input
  (:`Pressed`
    (set `self.index` 4)
    (goto _label))
  (:`Released`
    (set `self.index` 4)
    (goto _label_2)))

(event `UpdateHud`
  (bind _returnvalue (`self.GetHUD`))
  ;[1 1 1] Input
  (message `/Game/Blueprints/HUD/UIInterface.Setup` _returnvalue)
  (message `/Game/Blueprints/HUD/UIInterface.OnAmmoChanged` _returnvalue 20)
  (message `/Game/Blueprints/HUD/UIInterface.OnHealthChanged` _returnvalue 20.0))

(event `InputAction|QuickBar6`
  ;[1 1 1] Input
  (:`Pressed`
    (set `self.index` 5)
    (goto _label))
  (:`Released`
    (set `self.index` 5)
    (goto _label_2)))

(event `InputAction|QuickBar7`
  ;[1 1 1] Input
  (:`Pressed`
    (set `self.index` 6)
    (goto _label))
  (:`Released`
    (set `self.index` 6)
    (goto _label_2)))

(event `Key|P`
  ;[1 1 1] Create Spell window
  (:`Pressed`
    (`/Engine/EditorBlueprintResources/StandardMacros.IsValid` (`self.SpellWindow`)
      (:`Is Valid`
        (`self.RemoveSpellSheet`))
      (:`Is Not Valid`
        (`self.DisplaySpellSheet`)))))

(event `Key|G`
  (:`Pressed`
    (bind _asmy_char (`self.GetMyChar`))
    (`/Game/Blueprints/Weapons/Weaponbase.ServerUnEquip` (`/Game/Blueprints/MyChar.PrimaryWeapon` _asmy_char))))

(fn `DisplaySpellSheet`
  (bind _returnvalue (`|CreateWidget` "/Game/Blueprints/Spells/SpellSheet.SpellSheet_C"))
  (bind _output_get (set `self.SpellWindow` _returnvalue))
  (`/Game/Blueprints/Spells/SpellSheet.InitSpellSheet` _output_get self)
  (`UserWidget.AddToViewport` _output_get 0)
  (`WidgetBlueprintLibrary.SetInputMode_UIOnlyEx` null _output_get true)
  (set `self.bShowMouseCursor` true)
  (`WidgetBlueprintLibrary.SetFocusToGameViewport`))

(fn `HasSpellToUse`
  (returns (Item :type "/Game/Blueprints/Spells/SpellDetails Structure") (canUse :type Boolean))
  ;[1 1 1] If we have any spells
  (set `self.canUseSpell` (> (`KismetArrayLibrary.Array_Length` (`self.PlayerSpells`)) 0))
  ;[1 1 1] If we have a spell in that slot
  (bind _output_get (set `self.canUseSpell` (< (`self.Index`) (`KismetArrayLibrary.Array_Length` (`self.PlayerSpells`)))))
  (return (`KismetArrayLibrary.Array_Get` (`self.PlayerSpells`) (`self.Index`)) _output_get))

(fn `RemoveSpellSheet`
  (`Widget.RemoveFromParent` (`self.SpellWindow`))
  (set `self.SpellWindow` null)
  (`WidgetBlueprintLibrary.SetInputMode_GameOnly` null)
  (set `self.bShowMouseCursor` false)
  (`WidgetBlueprintLibrary.SetFocusToGameViewport`))

(fn `SetPlayerSpells`
  (params (Spells :type "Array of /Game/Blueprints/Spells/SpellDetails Structure"))
  (bind _output_get (set `self.PlayerSpells` Spells))
  (message `/Game/Blueprints/HUD/UIInterface.OnSetSpellBar` (`self.GetHUD`) _output_get))

(fn `UserConstructionScript`)