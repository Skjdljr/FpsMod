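; Base projectile actor that damages whatever it hits, with its instigator's controller credited for the damage.
; BeginPlay binds the actor hit event, which applies Damage with DamageType, destroys the projectile and prints the hit component's name for debugging.
; A separate ApplyMyDamage function, not called within this Blueprint, damages every Pawn overlapping a sphere sized to the collision radius, without passing DamageType.
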(event `self.ReceiveBeginPlay`
  (add `self.OnActorHit` (delegate `OnActorHit_Event_0`)))

(event `OnActorHit_Event_0` :!signature `self.OnActorHit`
  (params (SelfActor :type "Actor Object Reference") (OtherActor :type "Actor Object Reference") (NormalImpulse :type "Object.Vector Structure") (Hit :type "EngineTypes.HitResult Structure (by ref)"))
  (`GameplayStatics.ApplyDamage` OtherActor (`self.Damage`) (`self.GetInstigatorController`) self "/Script/Engine.DamageType")
  (`self.K2_DestroyActor`)
  (`KismetSystemLibrary.PrintString` (`KismetStringLibrary.BuildString_Name` "" "component name: " (`KismetStringLibrary.Conv_StringToName` (`KismetSystemLibrary.GetDisplayName` Hit_HitComponent)))))

(event `self.ReceiveTick`
  (params (DeltaSeconds :type "Float (single-precision)")))

(fn `ApplyMyDamage`
  (bind _outactors (`KismetSystemLibrary.SphereOverlapActors_NEW` (0.0 0.0 0.0) (`SphereComponent.SphereRadius` (`self.SphereCollison`)) (`|MakeArray` "ObjectTypeQuery3" :!type "EngineTypes.EObjectTypeQuery Enum")))
  (for _array_element _outactors
    (`GameplayStatics.ApplyDamage` _array_element (`self.Damage`) (`self.GetInstigatorController`) self)))

(fn `UserConstructionScript`)