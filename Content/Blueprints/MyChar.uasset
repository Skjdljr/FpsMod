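; MyChar is a networked player character with movement, sprinting, weapon fire, spells, health, ammo and color changes.
; Held left mouse calls the weapon's server shoot each Tick through a gate; the character's own projectile and spell functions spawn on authority, with cooldown checks stubbed true.
; Authority handles damage, refilling health at zero, and pushes changes to the HUD.
; Dropping a weapon destroys and respawns it to work around static mesh replication.
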(event Custom|Sprint
  (Variables|/Script/Engine.CharacterMovementComponent|SetMaxWalkSpeed (Variables|Character|GetCharacterMovement) 5e+02))

(event Custom|ChangeColorFromServer
  ;[0.09911 1 0.9618] Random Change color
  (bind _outactors (Actor|GetAllActorsOfClass "MyChar_C"))
  (for _array_element _outactors
    (bind _asmy_char (Utilities|Casting|CastToMyChar _array_element))
    (CallFunction|ChangeColor _asmy_char (Utilities|Array|Get(acopy) (Variables|Body|GetColorArray)))))

(event Custom|ServerAttemptShoot
  ;[0.02871 0.9522 1] Server calls
  ;;[1 1 1] Server AttemptShoot
  (Gun|AttemptShoot))

(event Custom|UpdateHealth
  (params (Health :type Float%20%28single-precision%29 :default 0.0))
  ;[0.04868 0.1098 1] Update HUD Calls Client Only
  (bind _asmy_hud (Utilities|GetMyhud)
    (:then
      (Class|UIInterface|OnHealthChanged(Message) _asmy_hud Health))))

(event Custom|Walk
  (Variables|/Script/Engine.CharacterMovementComponent|SetMaxWalkSpeed (Variables|Character|GetCharacterMovement) 2e+02))

(event Custom|DestroyItemOnServer
  (params (Item :type Actor%20Object%20Reference))
  ;[1 1 1] UGLY! Because replication is wonky with static mesh components just delete and respawn at current location
  (Networking|SwitchHasAuthority
    (:Authority
      (bind _asactor (Utilities|Casting|CastToActorClass (Utilities|GetClass Item)))
      (Game|SpawnActorfromClass _asactor (Transformation|GetActorTransform Item) false 0)
      (Actor|DestroyActor Item))))

(event Custom|DisplayHit
  (params (HitLocation :type Vector :default "0, 0, 0"))
  (Effects|SpawnEmitteratLocation "/Game/StarterContent/Particles/P_Explosion.P_Explosion" HitLocation)
  (CallFunction|PlayHitSound))

(event Custom|UpdateAmmo
  (params (ammo :type Integer :default 0))
  ;[0.04868 0.1098 1] Update HUD Calls Client Only
  (bind _asmy_hud (Utilities|GetMyhud)
    (:then
      (Default|OnAmmoChanged _asmy_hud ammo))))

(event Custom|ServerAttemptToUseSpell
  (params (Spell :type Spell%20Details%20Structure))
  ;[0.02871 0.9522 1] Server calls
  (Spells|CanUseSpell Spell)
  (Spells|AttemptSpell Spell))

(event EventTick
  (params (DeltaSeconds :type Float%20%28single-precision%29))
  ;[1 0.9087 0] Ask server to shoot
  (Utilities|FlowControl|Gate true
    (:Exit
      (Default|ServerAttemptShoot (Variables|Default|GetPrimaryWeapon)))))

(event EventBeginPlay
  ;[1 1 1] init
  (CallFunction|ChangeColor)
  (Attribute|InitAttributes))

(event EventPossessed
  (params (NewController :type Controller%20Object%20Reference))
  (Utilities|Casting|CastToMyPlayerController NewController))

(event EventAnyDamage
  (params (Damage :type Float%20%28single-precision%29) (DamageType :type Damage%20Type%20Object%20Reference) (InstigatedBy :type Controller%20Object%20Reference) (DamageCauser :type Actor%20Object%20Reference))
  ;[0.11 0.01638 0.01428] Take damage
  (if (!= InstigatedBy (Game|GetInstigatorController))
    (CallFunction|DisplayHit (Transformation|GetActorLocation DamageCauser))
    (CallFunction|OnTakeDamage Damage)))

(event Input|ActionEvents|InputActionRun
  (:Pressed
    (CallFunction|Sprint))
  (:Released
    (CallFunction|Walk)))

(event Input|ActionEvents|InputActionJump
  ;[1 1 1 0.3] Movement
  (:Pressed
    (Character|Jump)))

(event Input|AxisEvents|InputAxisMoveRight
  (params (AxisValue :type Float%20%28single-precision%29))
  ;[1 1 1 0.3] Movement
  (Pawn|Input|AddMovementInput (Math|Vector|GetRightVector (Transformation|GetActorRotation)) AxisValue false))

(event Input|AxisEvents|InputAxisMoveForward
  (params (AxisValue :type Float%20%28single-precision%29))
  ;[1 1 1 0.3] Movement
  (Pawn|Input|AddMovementInput (Math|Vector|GetForwardVector (Transformation|GetActorRotation)) AxisValue false))

(event Input|AxisEvents|InputAxisTurn
  (params (AxisValue :type Float%20%28single-precision%29))
  ;[1 1 1 0.3] Movement
  (Pawn|Input|AddControllerYawInput AxisValue))

(event Input|AxisEvents|InputAxisLookUp
  (params (AxisValue :type Float%20%28single-precision%29))
  ;[1 1 1 0.3] Movement
  (Pawn|Input|AddControllerPitchInput (* AxisValue -1.0)))

(event Input|MouseEvents|LeftMouseButton
  ;[1 0.9087 0] Ask server to shoot
  (:Pressed
    (Utilities|FlowControl|Gate true) ; enters at Open
  )
  (:Released
    (Utilities|FlowControl|Gate true) ; enters at Close
  ))

(event Input|KeyboardEvents|G
  (bind _primaryweapon (Variables|Default|GetPrimaryWeapon))
  (:Pressed
    (Utilities|IsValid _primaryweapon
      (:Is%20Valid
        (Default|ServerUnequip _primaryweapon)
        (CallFunction|DestroyItemonServer _primaryweapon)))))

(event Input|KeyboardEvents|F7
  ;[0.09911 1 0.9618] Random Change color
  (:Pressed
    (Networking|SwitchHasAuthority
      (:Authority
        (CallFunction|ChangeColorfromServer)))))

(fn ConstructionScript
  (bind _returnvalue (Rendering|Material|CreateDynamicMaterialInstance (Variables|Character|GetMesh) 0 0 :!class /Script/Engine.PrimitiveComponent))
  (Variables|Body|SetBody%20MID _returnvalue)
  (Variables|/Script/Engine.CharacterMovementComponent|SetMaxWalkSpeed (Variables|Character|GetCharacterMovement) (Variables|Attribute|GetMoveSpeed)))

(fn ChangeColor
  (params (New%20Color :type Linear%20Color%20Structure))
  (Rendering|Material|SetVectorParameterValue (Variables|Body|GetBody%20MID) (Variables|Body|GetColorMaterialName) New%20Color :!class /Script/Engine.MaterialInstanceDynamic))

(fn OnTakeDamage
  (params (Damage :type Float%20%28single-precision%29 :default 0.0))
  (Networking|SwitchHasAuthority
    (:Authority
      (bind _output_get (Variables|Attribute|Sethealth (- (Variables|Attribute|Gethealth) Damage)))
      (if (> _output_get 0.0)
        _
        (else
          (Development|PrintString "You have died, and are reborn!")
          (Attribute|InitHealth)))
      (CallFunction|UpdateHealth _output_get))))

(fn InitAttributes
  (Networking|SwitchHasAuthority
    (:Authority
      (Gun|InitAmmo)
      (Attribute|InitHealth))))

(fn OnRepHealth
  (Rendering|Components|TextRender|SetText (Variables|Default|GetMyHealthText) (Utilities|String|BuildString(Float) "" "Health: " (Variables|Attribute|Gethealth))))

(fn HasAmmo
  (return (> (Variables|Projectiles|GetAmmoCount) 0)))

(fn InitHealth
  (Networking|SwitchHasAuthority
    (:Authority
      (Variables|Attribute|Sethealth (Variables|Attribute|GetMaxHealth)))))

(fn InitAmmo
  (Networking|SwitchHasAuthority
    (:Authority
      (Variables|Projectiles|SetAmmoCount (Variables|Projectiles|GetMaxAmmoCount)))))

(fn AttemptShoot
  (Audio|PlaySoundatLocation "/Game/Assets/WeaponFire.FirstPerson_WeaponFire" (Transformation|GetActorLocation))
  (Networking|SwitchHasAuthority
    (:Authority
      (bind _hasammo (Attribute|HasAmmo))
      (if _hasammo
        (bind _returnvalue (CallFunction|GetForwardTransform))
        (Game|SpawnActorfromClass (Variables|Projectiles|GetProjectileClass) _returnvalue true self)
        (bind _output_get (Variables|Projectiles|SetAmmoCount (- (Variables|Projectiles|GetAmmoCount) 1)))
        (CallFunction|UpdateAmmo _output_get)))))

(fn PlayHitSound
  (bind _asmy_hud (Utilities|GetMyhud)
    (:then
      (Class|UserWidget|PlaySound (Variables|/Game/Blueprints/HUD/MyHUD.MyHUD_C|GetMyUI _asmy_hud) "/Game/StarterContent/Audio/Explosion_Cue.Explosion_Cue"))))

(fn CheckCoolDown
  (params (Spel :type Spell%20Details%20Structure))
  (return true))

(fn AttemptSpell
  (params (Spell :type Spell%20Details%20Structure))
  (Networking|SwitchHasAuthority
    (:Authority
      (bind (_canuse _spell) (Spells|CanUseSpell Spell))
      (if _canuse
        (Spells|MakeSpell _spell)))))

(fn CanUseSpell
  (params (spellToUse :type Spell%20Details%20Structure))
  (bind _notimeremains (Spells|CheckCoolDown spellToUse))
  (bind _output_get (LocalVariables|SetbCanUse _notimeremains))
  (return _output_get spellToUse))

(fn GetForwardTransform
  (return (Math|Transform|MakeTransform (+ (.location (Transformation|GetWorldTransform)) (Math|Vector|GetForwardVector (Variables|Default|GetArrowComponent))) (Pawn|GetControlRotation :!class /Script/Engine.Pawn) "1,1.000000,1")))

(fn MakeSpell
  (params (SpellDeets :type Spell%20Details%20Structure))
  (bind _returnvalue (CallFunction|GetForwardTransform))
  (Game|SpawnActorfromClass "/Game/Blueprints/Spells/BaseSpell.BaseSpell_C" _returnvalue true self))

(fn SetWeapon
  (params (Weapon :type Weapon%20Base%20Object%20Reference))
  (Variables|Default|SetPrimaryWeapon Weapon))

(fn HasWeaponEquiped
  (bind _primaryweapon (Variables|Default|GetPrimaryWeapon))
  (Utilities|IsValid _primaryweapon
    (:Is%20Valid
      (bind _attached (Default|IsAttachedtoPawn _primaryweapon))
      (return _attached))
    (:Is%20Not%20Valid
      (Development|PrintString "Weapon not valid"))))