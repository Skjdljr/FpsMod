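; MyHUD is the player HUD: it creates the MyUI widget and draws a textured crosshair.
; On BeginPlay it adds the widget to the viewport with a Server or Client title, and removes it on Destroyed.
; UI interface events pass quickbar input, health, ammo and spell slot or spellbar changes straight to the widget.
; DrawHUD renders the crosshair from the screen's center coordinates each frame.
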(event `self.ReceiveBeginPlay`
  (`self.Setup`))

(event `self.ReceiveDestroyed`
  (bind _myui (`self.MyUI`))
  (`/Engine/EditorBlueprintResources/StandardMacros.IsValid` _myui
    (:`Is Valid`
      (`Widget.RemoveFromParent` _myui))))

(event `self.Setup`
  (`/Engine/EditorBlueprintResources/StandardMacros.IsValid` (`self.MyUI`)
    (:`Is Not Valid`
      (bind _returnvalue (`|CreateWidget` "/Game/Blueprints/HUD/MyUI.MyUI_C"))
      (bind _output_get (set `self.MyUI` _returnvalue))
      (`UserWidget.AddToViewport` _output_get 0)
      (if (`KismetSystemLibrary.IsServer`)
        (bind _title (`/Game/Blueprints/HUD/MyUI.Title` _output_get))
        (`TextBlock.SetText` _title "Server")
        (else
          (`TextBlock.SetText` _title "Client"))))))

(event `self.QuickBarPressed`
  (params (Index :type Integer))
  ;[1 1 1] Ui Interface implementation calls
  (`/Game/Blueprints/HUD/MyUI.UseQuickBar` (`self.MyUI`) Index))

(event `self.ReceiveDrawHUD`
  (params (SizeX :type Integer) (SizeY :type Integer))
  ;[1 1 1] Draw cross hair
  (`self.DrawTexture` "/Game/Assets/Crosshair.FirstPersonCrosshair" (`KismetMathLibrary.Conv_IntToDouble` (/ SizeX 2)) (`KismetMathLibrary.Conv_IntToDouble` (/ SizeY 2)) 16.0 16.0 0.0 0.0 1.0 1.0))

(event `self.QuickBarReleased`
  (params (Index :type Integer))
  ;[1 1 1] Ui Interface implementation calls
  (`/Game/Blueprints/HUD/MyUI.ReleaseQuickbar` (`self.MyUI`) Index))

(event `self.OnHealthChanged`
  (params (health :type "Float (single-precision)"))
  ;[1 1 1] Ui Interface implementation calls
  (`/Game/Blueprints/HUD/MyUI.SetHealthText` (`self.MyUI`) health))

(event `self.OnAmmoChanged`
  (params (Ammo :type Integer))
  ;[1 1 1] Ui Interface implementation calls
  (`/Game/Blueprints/HUD/MyUI.SetAmmoText` (`self.MyUI`) Ammo))

(event `self.OnSetSpellSlot`
  (params (spell :type "/Game/Blueprints/Spells/SpellDetails Structure") (index :type Integer))
  ;[1 1 1] Ui Interface implementation calls
  (`/Game/Blueprints/HUD/MyUI.SetSpellSlot` (`self.MyUI`) spell index))

(event `self.OnSetSpellBar`
  (params (spells :type "Array of /Game/Blueprints/Spells/SpellDetails Structure (by ref)"))
  ;[1 1 1] Ui Interface implementation calls
  (`/Game/Blueprints/HUD/MyUI.SetSpellbar` (`self.MyUI`) spells))

(event `self.OnRefreshSpellbar`
  (params (spells :type "Array of /Game/Blueprints/Spells/SpellDetails Structure (by ref)"))
  ;[1 1 1] Ui Interface implementation calls
  (`/Game/Blueprints/HUD/MyUI.RefreshSkillBar` (`self.MyUI`) spells))

(fn `UserConstructionScript`)